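; BP_RootSpawner procedurally grows a chain of random spline prefab actors toward LevelGoal at BeginPlay.
; Each new piece spawns at the end transform of the previous piece's spline, repeating after SpawnDelay until that end passes the goal's X position.
; A downward line trace ignoring spawned pieces picks from UpSplinePrefabs when something lies within range below, otherwise from the regular SplinePrefabs.
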(event `self.ReceiveBeginPlay`
  (bind _spawnedsplineprefabs (`self.SpawnedSplinePrefabs`))
  (bind _outitem (`KismetArrayLibrary.Array_Random` (`self.SplinePrefabs`)))
  (bind _returnvalue (`self.GetComponentByClass` (`|GetArrayItem` _spawnedsplineprefabs (`KismetArrayLibrary.Array_LastIndex` _spawnedsplineprefabs)) "/Script/Engine.SplineComponent"))
  (bind _returnvalue_2 (`SplineComponent.GetNumberOfSplinePoints` _returnvalue))
  (bind _returnvalue_3 (`SplineComponent.GetLocationAtSplinePoint` _returnvalue _returnvalue_2 "World"))
  (bind _returnvalue_4 (`KismetMathLibrary.MakeTransform` _returnvalue_3 (`SplineComponent.GetRotationAtSplinePoint` _returnvalue _returnvalue_2 "World")))
  (`|ExecutionSequence`
    (:`then_0`
      (bind _returnvalue_5 (`|SpawnActorFromClass` _outitem (`self.GetTransform`) "Undefined" "OverrideRootScale" null null))
      (`KismetArrayLibrary.Array_Add` _spawnedsplineprefabs _returnvalue_5)
      (bind _returnvalue_6 (`|SpawnActorFromClass` _outitem _returnvalue_4 "Undefined" "OverrideRootScale" null null :!label _label))
      (`KismetArrayLibrary.Array_Add` (`self.SpawnedSplinePrefabs`) _returnvalue_6)
      (if (< (`KismetMathLibrary.BreakVector3f` (.location _returnvalue_4)) (.x (`self.K2_GetActorLocation` (`self.LevelGoal`)))) :!label _label_2
        (`KismetSystemLibrary.Delay` (`self.SpawnDelay`))
        (bind (_outhit _returnvalue_7) (`KismetSystemLibrary.LineTraceSingle` _returnvalue_3 (- _returnvalue_3 (0.0 0.0 5000.0)) "TraceTypeQuery1" false (`self.SpawnedSplinePrefabs`)))
        (if _returnvalue_7
          (bind _returnvalue_8 (`|SpawnActorFromClass` (`KismetArrayLibrary.Array_Random` (`self.UpSplinePrefabs`)) _returnvalue_4 "Undefined" "OverrideRootScale" null null))
          (`KismetArrayLibrary.Array_Add` (`self.SpawnedSplinePrefabs`) _returnvalue_8)
          (goto _label_2)
          (else
            (goto _label)))))))

(fn `UserConstructionScript`)
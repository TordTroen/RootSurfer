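; BP_SurfPlayerCharacter is the player character Blueprint that adds audio and visual feedback to movement events.
; Grapple hits, slides, jumps and landings play 2D sounds, with grapple hits also spawning a pooled Niagara dirt effect.
; Speed level changes select or stop the wind loop and play running audio only when moving on the ground uncrouched.
; Landing and primary action only add debug prints beyond this, with no movement logic here.
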(event `self.ReceiveBeginPlay`)

(event `self.OnGrappleHit`
  (params (Location :type "Vector Structure"))
  (`GameplayStatics.PlaySound2D` "/Game/Audio/GRAPPLE_ATTACH_FX_.GRAPPLE_ATTACH_FX_" 1.0 1.0 0.0 null null)
  (`NiagaraFunctionLibrary.SpawnSystemAtLocation` "/Game/Niagara/NS_Dirt.NS_Dirt" Location (struct) (1.0 1.0 1.0) true true "AutoRelease"))

(event `self.OnBeginSlide`
  (`GameplayStatics.PlaySound2D` "/Game/Audio/SLIDE_FX_.SLIDE_FX_" 1.0 1.0 0.0 null null)
  (`AudioComponent.Stop` (`self.RunSoundComp`)))

(event `self.OnJumped`
  (`GameplayStatics.PlaySound2D` "/Game/Audio/JUMP_FX.JUMP_FX" 1.0 1.0 0.0 null null))

(event `self.OnLanded`
  (params (Hit :type "HitResult Structure (by ref)"))
  (`KismetSystemLibrary.PrintString` (`KismetSystemLibrary.GetDisplayName` (`.HitActor` (`GameplayStatics.BreakHitResult` Hit))))
  (`GameplayStatics.PlaySound2D` "/Game/Audio/LAND_FX.LAND_FX" 1.0 1.0 0.0 null null))

(event `self.OnSpeedLevelChange`
  (params (SpeedLevel :type Integer))
  (bind _windsoundcomp (`self.WindSoundComp`))
  (`|ExecutionSequence`
    (:`then_0`
      (switch `int` SpeedLevel
        (:`0`
          (`AudioComponent.Stop` (`self.WindSoundComp`)))
        (:`1`
          (`AudioComponent.SetSound` (`self.WindSoundComp`) "/Game/Audio/WIND_1_FX.WIND_1_FX")
          (`AudioComponent.Play` (`self.WindSoundComp`) 0.0 :!label _label))
        (:`2`
          (`AudioComponent.SetSound` _windsoundcomp "/Game/Audio/WIND_2_FX.WIND_2_FX")
          (goto _label))
        (:`3`
          (`AudioComponent.SetSound` _windsoundcomp "/Game/Audio/WIND_3_FX.WIND_3_FX")
          (goto _label))))
    (:`then_1`
      (if (and (> SpeedLevel 0) (not (`NavMovementComponent.IsCrouching` (`self.CharacterMovement`))) (`NavMovementComponent.IsMovingOnGround` (`self.CharacterMovement`)))
        (`AudioComponent.Play` (`self.RunSoundComp`) 0.0)
        (else
          (`AudioComponent.Stop` (`self.RunSoundComp`)))))))

(event `self.OnPrimaryAction`
  (`KismetSystemLibrary.PrintString` "Primary action"))

(fn `UserConstructionScript`)